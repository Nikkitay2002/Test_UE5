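; BP_Player is the player's Blueprint, whose Player component reacts to contact with AI actors and other collisions.
; Overlapping an AI_Main_Father repaints its Cube with BallMaterial and calls Finish, identically whether or not it wore M_Target.
; Any hit on the component sets Jump to true on BP_Controller, with no ground check.
; Color-message interface calls, target/cleaner casts and several helper nodes are left unconnected.
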(event OnComponentHit(Player)
  (params (HitComponent :type Primitive%20Component%20Object%20Reference) (OtherActor :type Actor%20Object%20Reference) (OtherComp :type Primitive%20Component%20Object%20Reference) (NormalImpulse :type Vector :default "0, 0, 0") (Hit :type Hit%20Result%20Structure%20%28by%20ref%29))
  (if true
    (bind _asbp_controller (Utilities|Casting|CastToBP_Controller (Game|GetPlayerController 0)))
    (Variables|/Game/Player_Control/BP_Controller.BP_Controller_C|SetJump _asbp_controller true)))

(event OnComponentBeginOverlap(Player)
  (params (OverlappedComponent :type Primitive%20Component%20Object%20Reference) (OtherActor :type Actor%20Object%20Reference) (OtherComp :type Primitive%20Component%20Object%20Reference) (OtherBodyIndex :type Integer) (bFromSweep :type Boolean) (SweepResult :type Hit%20Result%20Structure%20%28by%20ref%29))
  (bind _asai_main_father (Utilities|Casting|CastToAI_Main_Father OtherActor))
  (if (== (Rendering|Material|GetMaterial (Variables|/Game/AI/Father/AI_Main_Father.AI_Main_Father_C|GetCube _asai_main_father) 0) "/Game/AI/Target/M_Target.M_Target")
    (Rendering|Material|SetMaterial (Variables|/Game/AI/Father/AI_Main_Father.AI_Main_Father_C|GetCube _asai_main_father) 0 (Variables|Default|GetBall_Material))
    (bind _asai_main_father_2 (Utilities|Casting|CastToAI_Main_Father OtherActor))
    (Default|Finish _asai_main_father_2)
    (else
      (Rendering|Material|SetMaterial (Variables|/Game/AI/Father/AI_Main_Father.AI_Main_Father_C|GetCube _asai_main_father) 0 (Variables|Default|GetBall_Material))
      (bind _asai_main_father_3 (Utilities|Casting|CastToAI_Main_Father OtherActor))
      (Default|Finish _asai_main_father_3))))

(event EventBeginPlay)

(event Input|KeyboardEvents|SpaceBar
  (params (Key :type Key%20Structure :default "None")))

(fn ConstructionScript)

(fn NewFunction
  (return (or false false)))

(fn OnRepChTarget)
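; BP_Controller is a player controller that drives a physics-based BP_Player, cached from the controlled pawn on BeginPlay.
; Each tick, held WASD keys apply mass-independent forces to the Player component along the camera's forward and right vectors.
; Mouse axes feed yaw and inverted pitch input.
; Space plays a sound and adds an upward velocity impulse, gated by a Jump flag that this graph clears but never resets.
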(event EventBeginPlay
  (bind _asbp_player (Utilities|Casting|CastToBP_Player (Pawn|GetControlledPawn)))
  (Variables|Default|SetBP%20Player _asbp_player))

(event EventTick
  (params (DeltaSeconds :type Float%20%28single-precision%29))
  (bind _bp_player (Variables|Default|GetBP%20Player))
  (bind _bp_player_2 (Variables|Default|GetBP%20Player))
  (bind _bp_player_3 (Variables|Default|GetBP%20Player))
  (bind _bp_player_4 (Variables|Default|GetBP%20Player))
  (Utilities|FlowControl|Sequence
    (:then_0
      (if (Game|Player|IsInputKeyDown "W")
        (Physics|AddForce (Variables|/Game/Player_Control/BP_Player.BP_Player_C|GetPlayer _bp_player_4) (* (Math|Vector|GetForwardVector (Variables|/Game/Player_Control/BP_Player.BP_Player_C|GetCamera _bp_player_4)) 1e+03) "None" true)))
    (:then_1
      (if (Game|Player|IsInputKeyDown "S")
        (Physics|AddForce (Variables|/Game/Player_Control/BP_Player.BP_Player_C|GetPlayer _bp_player) (* (Math|Vector|GetForwardVector (Variables|/Game/Player_Control/BP_Player.BP_Player_C|GetCamera _bp_player)) -1e+03) "None" true)))
    (:then_2
      (if (Game|Player|IsInputKeyDown "A")
        (Physics|AddForce (Variables|/Game/Player_Control/BP_Player.BP_Player_C|GetPlayer _bp_player_2) (* (Math|Vector|GetRightVector (Variables|/Game/Player_Control/BP_Player.BP_Player_C|GetCamera _bp_player_2)) -1e+03) "None" true)))
    (:then_3
      (if (Game|Player|IsInputKeyDown "D")
        (Physics|AddForce (Variables|/Game/Player_Control/BP_Player.BP_Player_C|GetPlayer _bp_player_3) (* (Math|Vector|GetRightVector (Variables|/Game/Player_Control/BP_Player.BP_Player_C|GetCamera _bp_player_3)) 1e+03) "None" true)))))

(event Input|ActionEvents|InputActionjump
  (params (Key :type Key%20Structure :default "None")))

(event Input|MouseEvents|MouseX
  (params (AxisValue :type Float%20%28single-precision%29))
  (Class|PlayerController|AddYawInput AxisValue))

(event Input|MouseEvents|MouseY
  (params (AxisValue :type Float%20%28single-precision%29))
  (Class|PlayerController|AddPitchInput (* AxisValue -1.0)))

(event Input|KeyboardEvents|SpaceBar
  (params (Key :type Key%20Structure :default "None"))
  (:Pressed
    (if (Variables|Default|GetJump)
      (Variables|Default|SetJump false)
      (Audio|SpawnSound2D "/Game/Sounds/Ball_Jump.Ball_Jump" 1.0 1.0 0.0 0)
      (Physics|AddImpulse (Variables|/Game/Player_Control/BP_Player.BP_Player_C|GetPlayer (Variables|Default|GetBP%20Player)) "0.000000,0.000000,1000.000000" "None" true))))

(fn ConstructionScript)